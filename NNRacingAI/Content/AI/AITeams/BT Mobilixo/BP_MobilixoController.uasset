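; AI controller for the Mobilixo team's race car, which starts driving on RaceStarted with a timed head start.
; Each tick, a speed-scaled forward trace sets throttle and brake, while angled side traces sum into steering, accounting for slippery surfaces.
; A downward trace detects leaving the track, switching steering toward the last on-track position.
; A torque impulse handles flipped cars; spline and edge-material steering helpers are not called here.
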(event Custom|ResetHead
  (Variables|Default|SetHeadStart false))

(event EventBeginPlay
  (bind _outactors (Actor|GetAllActorsOfClass "/Script/Engine.Pawn"))
  (Variables|Default|SetignoreActors _outactors)
  (bind _returnvalue (Actor|GetActorOfClass "/Game/VehicleTemplate/Blueprints/Track.Track_C"))
  (Variables|Default|SetTrackRef _returnvalue))

(event EventTick
  (params (DeltaSeconds :type Float%20%28single-precision%29))
  (Development|PrintString (Utilities|String|Append "Vehicle Velocity" (Utilities|String|ToString(Float) (Utilities|GetVehicleVelocity))) true true "(R=1.000000,G=0.033720,B=0.000000,A=1.000000)" 0.0)
  (bind _returnvalue (CallFunction|IsInsidetheTrack))
  (Development|PrintString (Utilities|String|Append "Is Inside Track: " (Utilities|String|ToString(Boolean) _returnvalue)) true true "(R=1.000000,G=0.232926,B=0.256803,A=1.000000)" 0.0)
  (if _returnvalue
    (Utilities|FlowControl|Sequence
      (:then_0
        ;[1 1 1] Throttle & Break
        (bind (_outhit _tracedistance) (CallFunction|ForwardTraceCheck false :!label _label))
        (bind _returnvalue_2 (CallFunction|ShouldIgnoreTrackEdge (.HitComponent (Collision|BreakHitResult _outhit))))
        (if _returnvalue_2
          _
          (else
            _))
        (if (Utilities|ShouldBreak (.bBlockingHit (Collision|BreakHitResult _outhit)) (.Distance (Collision|BreakHitResult _outhit)))
          (if (> (- 1.0 (/ (.Distance (Collision|BreakHitResult _outhit)) _tracedistance)) 0.5)
            (CallFunction|BreakVehicle (Utilities|BreakCalc (- 1.0 (/ (.Distance (Collision|BreakHitResult _outhit)) _tracedistance))))
            (Development|PrintString (Utilities|String|Append "Break val: " (Utilities|String|ToString(Float) (Utilities|BreakCalc (- 1.0 (/ (.Distance (Collision|BreakHitResult _outhit)) _tracedistance))))) true true "(R=1.000000,G=0.674976,B=0.000000,A=1.000000)" 0.0)
            (else
              (CallFunction|BreakVehicle 0.0)))
          (bind _output_get (Variables|Default|SetThrottleForce (Utilities|ThrottleCalc (Math|Float|Clamp(Float) (/ (.Distance (Collision|BreakHitResult _outhit)) _tracedistance) 0.2))))
          (else
            (Variables|Default|SetThrottleForce 1.0)))
        (Development|PrintString (Utilities|String|Append "Throttle " (Utilities|String|ToString(Float) _output_get)) true true "(R=0.000000,G=0.660000,B=1.000000,A=1.000000)" 0.0))
      (:then_1
        ;[1 1 1] Steer
        (Variables|Default|SetSteerVal 0.0)
        (for _array_element (Variables|Default|GetDirections)
          (bind (_outhit_2 _tracedistance_2) (CallFunction|RightTraceCheck _array_element false))
          (Variables|Default|SetSteerVal (+ (* (Math|Float|SelectFloat 1.0 (/ (.Distance (Collision|BreakHitResult _outhit_2)) _tracedistance_2) (== (.PhysMat (Collision|BreakHitResult _outhit_2)) (Variables|Default|GetSlippery))) (Math|Float|SelectFloat -1.0 1.0 (< _array_element 0.0))) (Variables|Default|GetSteerVal))))
        (CallFunction|SteerVehicle (* (+ (Variables|Default|GetSteerVal) (* (Variables|Default|GetSteerVal) (Variables|Default|GetThrottleForce))) 4.0))
        (Variables|Default|SetSteerVal (* (+ (Variables|Default|GetSteerVal) (* (Variables|Default|GetSteerVal) (Variables|Default|GetThrottleForce))) 4.0))
        (Development|PrintString (Utilities|String|Append "Steer : " (Utilities|String|ToString(Float) (* (+ (Variables|Default|GetSteerVal) (* (Variables|Default|GetSteerVal) (Variables|Default|GetThrottleForce))) 4.0))) true true "(R=1.000000,G=0.721922,B=0.000000,A=1.000000)" 0.0))
      (:then_2
        (Default|Throttle (Variables|Default|GetControlledCar) (Variables|Default|GetThrottleForce) :!label _label_2)
        (Development|PrintString (Utilities|String|Append "Real Force: " (Utilities|String|ToString(Float) 0.0)) true true "(R=0.000000,G=0.660000,B=1.000000,A=1.000000)" 0.0))
      (:then_3
        (Variables|Default|SetMyLastTrackPos (Transformation|GetActorLocation (Variables|Default|GetControlledCar))))
      (:then_4
        (CallFunction|CheckCarFlipped :!label _label_3)))
    (else
      (Utilities|FlowControl|Sequence
        (:then_0
          (goto _label))
        (:then_1
          (goto _label_2))
        (:then_2
          (CallFunction|SteertoLastTrackPos))
        (:then_3
          (goto _label_3))))))

(event EventPossess
  (params (PossessedPawn :type Pawn%20Object%20Reference))
  (Variables|Default|SetCar%20Color "(R=0.633333,G=0.028778,B=0.000000,A=1.000000)")
  (Variables|Default|SetTeam%20Name "Mobilixo")
  (|CallParentFunction PossessedPawn))

(event EventRaceStarted
  (bind _controlledcar (Variables|Default|GetControlledCar))
  (bind _returnvalue (Transformation|GetActorLocation _controlledcar))
  (Actor|Tick|SetActorTickEnabled true)
  (Variables|Default|SetHeadStart true)
  (Utilities|Time|SetTimerbyEvent (delegate Custom|ResetHead) (Variables|Default|GetHeadStartTime))
  (Utilities|FlowControl|Sequence
    (:then_0
      (bind _outactors (Actor|GetAllActorsOfClass "/Game/AI/AISportsCar_Pawn.AISportsCar_Pawn_C"))
      (|SetBy-RefVar (Variables|Default|GetignoreActors) _outactors))
    (:then_1
      (bind _outhit (Collision|LineTraceByChannel _returnvalue (* (* _returnvalue (Math|Vector|VectorDown)) (Math|Float|MakeLiteralFloat 2.1e+04)) "TraceTypeQuery1" false (Variables|Default|GetignoreActors) "ForDuration" true "(R=1.000000,G=0.000000,B=0.873856,A=1.000000)" "(R=0.000000,G=0.016063,B=1.000000,A=1.000000)"))
      (Variables|Default|SetGroundDistance (.Distance (Collision|BreakHitResult _outhit)))
      (Development|PrintString (Utilities|String|Append "Distance: " (Utilities|String|ToString(Float) (.Distance (Collision|BreakHitResult _outhit)))) true true "(R=1.000000,G=0.000000,B=0.135502,A=1.000000)"))))

(fn ConstructionScript
  (|CallParentFunction))

(fn GetSplinePointstoFollow
  (bind _returnvalue (Actor|GetActorOfClass "/Game/VehicleTemplate/Blueprints/Track.Track_C"))
  (for _index (range 0 (- (Spline|GetNumberOfSplinePoints (Variables|/Game/VehicleTemplate/Blueprints/Track.Track_C|GetSpline _returnvalue)) 1))
    (Utilities|Array|Add (LocalVariables|GetOutSplinePoints) (Utilities|Struct|MakeSplinePoint (Math|Conversions|ToFloat(Integer) _index) (.location (Spline|GetTransformatSplinePoint (Variables|/Game/VehicleTemplate/Blueprints/Track.Track_C|GetSpline _returnvalue) _index "World" true)) "0.000000,0.000000,0.000000" (Spline|GetTangentatSplinePoint (Variables|/Game/VehicleTemplate/Blueprints/Track.Track_C|GetSpline _returnvalue) _index "Local") (.rotation (Spline|GetTransformatSplinePoint (Variables|/Game/VehicleTemplate/Blueprints/Track.Track_C|GetSpline _returnvalue) _index "World" true)) (.scale (Spline|GetTransformatSplinePoint (Variables|/Game/VehicleTemplate/Blueprints/Track.Track_C|GetSpline _returnvalue) _index "World" true)) (Class|SplineComponent|GetSplinePointType (Variables|/Game/VehicleTemplate/Blueprints/Track.Track_C|GetSpline _returnvalue) _index))))
  (return (LocalVariables|GetOutSplinePoints) _returnvalue))

(fn ForwardTraceCheck
  (params (bDebugEnabled :type Boolean))
  (bind _returnvalue (Utilities|GetVehicleVelocity))
  (bind _controlledcar (Variables|Default|GetControlledCar))
  (bind _controlledcar_2 (Variables|Default|GetControlledCar))
  (bind _fronttracedistance (Variables|Default|GetFrontTraceDistance))
  (bind _returnvalue_2 (Transformation|GetActorForwardVector _controlledcar_2))
  (bind _returnvalue_3 (Transformation|GetActorForwardVector _controlledcar))
  (bind _returnvalue_4 (Transformation|GetActorLocation _controlledcar))
  (bind _returnvalue_5 (/ _returnvalue 1e+03))
  (bind _returnvalue_6 (* _fronttracedistance _returnvalue_5))
  (bind _returnvalue_7 (* _returnvalue_3 1e+02))
  (bind _returnvalue_8 (Math|Float|Clamp(Float) _returnvalue_6 _fronttracedistance 1e+70))
  (bind _returnvalue_9 (+ _returnvalue_4 _returnvalue_7))
  (bind _returnvalue_10 (* _returnvalue_2 _returnvalue_8))
  (bind _returnvalue_11 (+ _returnvalue_9 _returnvalue_10))
  (bind _outhit (Class|KismetSystemLibrary|LineTraceSinglebyProfile _returnvalue_9 (Math|Vector|MakeVector (.x _returnvalue_11) (.y _returnvalue_11) 0.0) "" true (Variables|Default|GetignoreActors) (select bDebugEnabled "ForOneFrame" "None") true))
  (return _outhit _returnvalue_8 (not (== (.PhysMat (Collision|BreakHitResult _outhit)) (Variables|Default|GetRoadPhysmat)))))

(fn RightTraceCheck
  (params (DirectionMultiplier :type Float%20%28double-precision%29) (bDebugEnabled :type Boolean))
  (bind _controlledcar (Variables|Default|GetControlledCar))
  (bind _checksteerdistance (Variables|CarParameters|GetCheckSteerDistance))
  (bind _controlledcar_2 (Variables|Default|GetControlledCar))
  (bind _returnvalue (Transformation|GetActorForwardVector _controlledcar_2))
  (bind _returnvalue_2 (Transformation|GetActorRightVector _controlledcar_2))
  (bind _returnvalue_3 (Transformation|GetActorForwardVector _controlledcar))
  (bind _returnvalue_4 (Transformation|GetActorRightVector _controlledcar))
  (bind _returnvalue_5 (Transformation|GetActorLocation _controlledcar))
  (bind _returnvalue_6 (* _returnvalue_4 0.45 DirectionMultiplier))
  (bind _returnvalue_7 (* _returnvalue_2 0.45 DirectionMultiplier))
  (bind _returnvalue_8 (+ _returnvalue_7 _returnvalue))
  (bind _returnvalue_9 (+ _returnvalue_6 _returnvalue_3))
  (bind _returnvalue_10 (* _returnvalue_9 1e+02))
  (bind _returnvalue_11 (* _returnvalue_8 _checksteerdistance))
  (bind _returnvalue_12 (+ _returnvalue_5 _returnvalue_10))
  (bind _returnvalue_13 (+ _returnvalue_12 _returnvalue_11))
  (bind _outhit (Class|KismetSystemLibrary|LineTraceSinglebyProfile _returnvalue_12 (Math|Vector|MakeVector (.x _returnvalue_13) (.y _returnvalue_13) 0.0) "" true (Variables|Default|GetignoreActors) (select bDebugEnabled "ForOneFrame" "None") true))
  (return _outhit (Math|Vector|Distance(Vector) (Math|Vector|MakeVector (.x _returnvalue_13) (.y _returnvalue_13) 0.0) _returnvalue_12)))

(fn RightSteerBasedonHitDistance
  (params (Hit :type Hit%20Result%20Structure%20%28by%20ref%29) (SteerDirectionMultiplier :type Integer))
  (bind (_bblockinghit _binitialoverlap _time _distance _location _impactpoint _normal _impactnormal _physmat _hitactor _hitcomponent _hitbonename _bonename _hititem _elementindex _faceindex _tracestart) (Collision|BreakHitResult Hit))
  (Utilities|IsValid _hitcomponent
    (:Is%20Valid
      (if (CallFunction|IsTrackEdgeMaterial _hitcomponent _faceindex)
        (CallFunction|SteerVehicle (CallFunction|CalculateSteering _impactpoint _tracestart SteerDirectionMultiplier))
        (return false)
        (else
          _)))
    (:Is%20Not%20Valid
      _))
  (return true))

(fn IsTrackEdgeMaterial
  (params (Component :type Primitive%20Component%20Object%20Reference) (FaceIndex :type Integer))
  (return (== (.ReturnValue (Class|PrimitiveComponent|GetMaterialfromCollisionFaceIndex Component FaceIndex)) "/Game/Track/MI_TrackEdge.MI_TrackEdge")))

(fn CalculateSteering
  (params (A :type Vector) (B :type Vector) (SteerDirectionMultiplier :type Integer))
  (return (Math|Float|MapRangeClamped (Math|Vector|VectorLength (- A B)) 0.0 (Variables|CarParameters|GetCheckSteerDistance) (* SteerDirectionMultiplier (Variables|CarParameters|GetMaxSteerValue)) (* SteerDirectionMultiplier (Variables|CarParameters|GetMinSteerValue)))))

(fn CalculateBreak
  (params (A :type Vector) (B :type Vector))
  (return (Math|Float|MapRangeClamped (Math|Vector|VectorLength (- A B)) 0.0 (Variables|CarParameters|GetCheckBrakeDistance) (Variables|CarParameters|GetMaxBrakeValue) (Variables|CarParameters|GetMinBrakeValue))))

(fn BreakVehicle
  (params (Action%20Value :type Float%20%28double-precision%29))
  (if (> (Vehicle|GetForwardSpeed (Variables|/Game/AI/AISportsCar_Pawn.AISportsCar_Pawn_C|GetChaos%20Wheeled%20Vehicle%20Movement%20Component (Variables|Default|GetControlledCar))) 6e+02)
    (Default|Break (Variables|Default|GetControlledCar) Action%20Value)
    (Variables|Default|SetbIsBraking true)
    (else
      (Variables|Default|SetbIsBraking false)
      (Default|Break (Variables|Default|GetControlledCar) 0.0))))

(fn SteerVehicle
  (params (Action%20Value :type Float%20%28double-precision%29))
  (if (> (Vehicle|GetForwardSpeed (Variables|/Game/AI/AISportsCar_Pawn.AISportsCar_Pawn_C|GetChaos%20Wheeled%20Vehicle%20Movement%20Component (Variables|Default|GetControlledCar))) 2e+02)
    (Default|Steering (Variables|Default|GetControlledCar) Action%20Value)
    (else
      (Default|Steering (Variables|Default|GetControlledCar) 0.0))))

(fn ResetCarSteerBreak
  (bind _controlledcar (Variables|Default|GetControlledCar))
  (Variables|Default|SetbIsBraking false)
  (Default|Steering _controlledcar 0.0)
  (Default|Break _controlledcar 0.0))

(fn TraceForwardTest
  (bind _returnvalue (Math|Float|MakeLiteralFloat 4e+03))
  (bind _grounddistance (Variables|Default|GetGroundDistance))
  (bind _controlledcar (Variables|Default|GetControlledCar))
  (bind _controlledcar_2 (Variables|Default|GetControlledCar))
  (bind _returnvalue_2 (Transformation|GetActorForwardVector _controlledcar))
  (bind _returnvalue_3 (Transformation|GetActorLocation _controlledcar_2))
  (bind _returnvalue_4 (Transformation|GetActorForwardVector _controlledcar_2))
  (bind _returnvalue_5 (Transformation|GetActorLocation _controlledcar))
  (bind _returnvalue_6 (- _grounddistance -1.0))
  (bind (_x _y) (Math|Vector|BreakVector _returnvalue_5))
  (bind _z (Math|Vector|BreakVector _returnvalue_3))
  (bind _returnvalue_7 (* _returnvalue_2 _returnvalue))
  (bind _returnvalue_8 (+ _returnvalue_3 _returnvalue_4))
  (bind _returnvalue_9 (Math|Vector|MakeVector _x _y 5.0))
  (bind _returnvalue_10 (- _z _returnvalue_6))
  (bind _returnvalue_11 (Math|Vector|MakeVector (.x _returnvalue_8) (.y _returnvalue_8) _returnvalue_10))
  (bind _returnvalue_12 (+ _returnvalue_9 _returnvalue_7))
  (bind _returnvalue_13 (Math|Float|Absolute(Float) (.z _returnvalue_12)))
  (bind _returnvalue_14 (Math|Vector|MakeVector (.x _returnvalue_12) (.y _returnvalue_12) _returnvalue_13))
  (bind _outhit (Collision|LineTraceByChannel _returnvalue_11 _returnvalue_14 "TraceTypeQuery1" true 0 "ForOneFrame" true "(R=0.367946,G=0.000000,B=1.000000,A=1.000000)" "(R=1.000000,G=0.000000,B=0.790222,A=1.000000)"))
  (Development|PrintString (Utilities|String|Append (Utilities|String|ToString(Vector) _returnvalue_14) " - " (Utilities|String|ToString(Vector) _returnvalue_11) " " (Utilities|GetDisplayName (.PhysMat (Collision|BreakHitResult _outhit)))) true true "(R=1.000000,G=0.000000,B=0.904543,A=1.000000)" 0.0))

(fn DownTraceCheck
  (bind _controlledcar (Variables|Default|GetControlledCar))
  (bind _returnvalue (Transformation|GetActorLocation _controlledcar))
  (bind _outhit (Class|KismetSystemLibrary|LineTraceSinglebyProfile _returnvalue (* (* _returnvalue (Math|Vector|VectorDown)) (Math|Float|MakeLiteralFloat 2.1e+04)) "" true (Variables|Default|GetignoreActors) "None" true))
  (return _outhit))

(fn IsInsidetheTrack
  (bind _outhit (CallFunction|DownTraceCheck))
  (return (== (.HitActor (Collision|BreakHitResult _outhit)) (Variables|Default|GetTrackRef))))

(fn ShouldIgnoreTrackEdge
  (params (Component :type Primitive%20Component%20Object%20Reference))
  (Utilities|IsValid Component
    (:Is%20Valid
      (bind _returnvalue (CallFunction|IsInsidetheTrack))
      (return (and (not _returnvalue) (CallFunction|IsTrackEdgeMaterial Component))))
    (:Is%20Not%20Valid
      (return false))))

(fn SteertoLastTrackPos
  (bind _controlledcar (Variables|Default|GetControlledCar))
  (bind _mylasttrackpos (Variables|Default|GetMyLastTrackPos))
  (bind _returnvalue (Transformation|GetActorTransform _controlledcar))
  (bind _returnvalue_2 (Math|Rotator|FindRelativeLookatRotation _returnvalue _mylasttrackpos))
  (bind _returnvalue_3 (>= (.yaw _returnvalue_2) 0.0))
  (Development|PrintString (Utilities|String|ToString(Float) (.yaw _returnvalue_2)) true true "(R=0.960527,G=0.000000,B=1.000000,A=1.000000)" 0.0)
  (if _returnvalue_3
    (if (and _returnvalue_3 (>= (.yaw _returnvalue_2) 1e+02))
      (CallFunction|SteerVehicle 1.0)
      (else
        (CallFunction|SteerVehicle 0.0)))
    (elif (<= (.yaw _returnvalue_2) -1e+02)
      (CallFunction|SteerVehicle -1.0)
      (else
        (CallFunction|SteerVehicle 0.0)))))

(fn CheckCarFlipped
  (if (and (>= (Math|Float|Absolute(Float) (.roll (Transformation|GetActorRotation (Variables|Default|GetControlledCar)))) 1.7e+02) (Variables|Default|GetbCanFlipCar))
    (Class|PrimitiveComponent|AddTorqueinDegrees (Variables|/Script/ChaosVehicles.WheeledVehiclePawn|GetMesh (Variables|Default|GetControlledCar)) (Math|Transform|TransformDirection (Transformation|GetActorTransform (Variables|Default|GetControlledCar)) (Math|Vector|MakeVector 5e+04 0.0 0.0)) "None" true)
    (Variables|Default|SetbCanFlipCar false)
    (Development|PrintString "Car Flipped!" true true "(R=0.000000,G=1.000000,B=0.127024,A=1.000000)")
    (return)
    (else
      (Variables|Default|SetbCanFlipCar true)
      (return))))